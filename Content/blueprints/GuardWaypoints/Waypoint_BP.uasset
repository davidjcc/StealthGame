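; Waypoint actor that links into a patrol chain for guards or other agents that follow waypoints.
; When a valid actor implementing WaypointInterface overlaps its collider, it sends that actor the assigned next waypoint and itself as the current one.
; An optional debug toggle draws a timed arrow from this waypoint toward the next.
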(event `self.Collider.OnComponentBeginOverlap`
  (params (OtherActor :type "Actor Object Reference") (OtherComp :type "PrimitiveComponent Object Reference") (OtherBodyIndex :type Integer) (bFromSweep :type Boolean) (SweepResult :type "EngineTypes.HitResult Structure (by ref)"))
  (`/Engine/EditorBlueprintResources/StandardMacros.IsValid` OtherActor
    (:`Is Valid`
      (`/Engine/EditorBlueprintResources/StandardMacros.IsValid` (`self.NextWaypoint`)
        (:`Is Valid`
          (if (`KismetSystemLibrary.DoesImplementInterface` OtherActor "/Game/blueprints/GuardWaypoints/WaypointInterface.WaypointInterface_C")
            (message `/Game/blueprints/GuardWaypoints/WaypointInterface.SetNextWaypoint` OtherActor (`self.NextWaypoint`) self)
            (if (`self.DrawDebugLine`)
              (`KismetSystemLibrary.DrawDebugArrow` (`self.K2_GetActorLocation`) (`self.K2_GetActorLocation` (`self.NextWaypoint`)) 1500.0 (struct :`A` 1.0) 10.0))))))))

(fn `UserConstructionScript`)