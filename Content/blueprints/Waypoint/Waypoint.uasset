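; Waypoint actor that links to a next waypoint, forming a path that overlapping actors can follow.
; When an actor implementing WaypointInterface overlaps the Collider, it receives the next waypoint and the current one through an interface message, provided a next waypoint is set.
; An optional debug arrow briefly shows the link to the next waypoint at that moment.
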(event `self.Collider.OnComponentBeginOverlap`
  (params (OtherActor :type "Actor Object Reference") (OtherComp :type "PrimitiveComponent Object Reference") (OtherBodyIndex :type Integer) (bFromSweep :type Boolean) (SweepResult :type "EngineTypes.HitResult Structure (by ref)"))
  (`/Engine/EditorBlueprintResources/StandardMacros.IsValid` OtherActor
    (:`Is Valid`
      (`/Engine/EditorBlueprintResources/StandardMacros.IsValid` (`self.NextWaypoint`)
        (:`Is Valid`
          (if (`KismetSystemLibrary.DoesImplementInterface` OtherActor "/Game/Blueprints/Waypoint/WaypointInterface.WaypointInterface_C")
            (message `/Game/Blueprints/Waypoint/WaypointInterface.SetNextWaypoint` OtherActor (`self.NextWaypoint`) self)
            (if (`self.DrawDebugLine`)
              (`KismetSystemLibrary.DrawDebugArrow` (`self.K2_GetActorLocation`) (`self.K2_GetActorLocation` (`self.NextWaypoint`)) 1500.0 (struct :`A` 1.0) 10.0))))))))

(fn `UserConstructionScript`)