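; Waypoint actor that, when another actor overlaps its collider, picks that actor's next waypoint by weighted random choice.
; Each overlap normalizes the Waypoints array weights, then walks it against a random float, though the running count adds raw rather than normalized weights.
; The pick is sent with this waypoint through WaypointInterface to the overlapping actor, with an optional debug arrow.
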(event `self.Collider.OnComponentBeginOverlap`
  (params (OtherActor :type "Actor Object Reference") (OtherComp :type "PrimitiveComponent Object Reference") (OtherBodyIndex :type Integer) (bFromSweep :type Boolean) (SweepResult :type "EngineTypes.HitResult Structure (by ref)"))
  (`/Engine/EditorBlueprintResources/StandardMacros.IsValid` OtherActor
    (:`Is Valid`
      (`|ExecutionSequence`
        (:`then_0`
          ;[1 1 1] Init variables
          (set `self.AccumulatedWeightValue` 0.0)
          (set `self.WeightCount` 0.0)
          (set `self.RandomValue` (`KismetMathLibrary.RandomFloat`))
          (set `self.NextWaypoint` null))
        (:`then_1`
          ;[1 1 1] Calculate accumulated weights
          (for _array_element (`self.Waypoints`)
            (set `self.AccumulatedWeightValue` (+ (`.Weight_7_D9B70E3E4BE2D6702D06EC850B4A756B` (break `/Game/Blueprints/Waypoint/WeightedActor` _array_element)) (`self.AccumulatedWeightValue`)))))
        (:`then_2`
          ;[1 1 1] Calculate normalized weight for each element in the array
          (for (_array_element_2 _array_index) (`self.Waypoints`)
            (bind (_actor _weight) (break `/Game/Blueprints/Waypoint/WeightedActor` _array_element_2))
            (`KismetArrayLibrary.Array_Set` (`self.Waypoints`) _array_index (make `/Game/Blueprints/Waypoint/WeightedActor` _actor _weight (/ _weight (`self.AccumulatedWeightValue`))))))
        (:`then_3`
          ;[1 1 1] Set which waypoint lies within the current random value range
          (for _array_element_3 (`self.Waypoints`)
            (bind (_actor_2 _weight_2 _normalizedweight) (break `/Game/Blueprints/Waypoint/WeightedActor` _array_element_3))
            (if (>= (+ _normalizedweight (`self.WeightCount`)) (`self.RandomValue`))
              (set `self.NextWaypoint` _actor_2)
              (break)
              (else
                (set `self.WeightCount` (+ _weight_2 (`self.WeightCount`))))))
          (`/Engine/EditorBlueprintResources/StandardMacros.IsValid` (`self.NextWaypoint`)
            (:`Is Valid`
              (if (`KismetSystemLibrary.DoesImplementInterface` OtherActor "/Game/Blueprints/Waypoint/WaypointInterface.WaypointInterface_C")
                (message `/Game/Blueprints/Waypoint/WaypointInterface.SetNextWaypoint` OtherActor (`self.NextWaypoint`) self)
                (if (`self.DrawDebugLine`)
                  (`KismetSystemLibrary.DrawDebugArrow` (`self.K2_GetActorLocation`) (`self.K2_GetActorLocation` (`self.NextWaypoint`)) 1500.0 (struct :`A` 1.0) 10.0))))))))))

(fn `UserConstructionScript`)