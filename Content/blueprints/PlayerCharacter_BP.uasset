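; Player character with a HUD, pause menu, stealth tagging and a teleport gadget.
; Left click spawns the gadget, then after a short delay teleports the player to it with steam bursts and destroys it.
; During the teleport the mesh swaps to a dissolve material, animated by Tick through a material parameter collection.
; Tick also swaps actor tags by IsInStealth, assigning NotStealthTags when it is true.
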(event `InputAction|GamePause`
  ;[1 1 1] Pause Game
  (:`Pressed`
    (`GameplayStatics.SetGamePaused` null true)
    (bind _returnvalue (`|CreateWidget` "/Game/UI/WBP_PauseMenu.WBP_PauseMenu_C"))
    (`UserWidget.AddToViewport` _returnvalue 0)
    (set `PlayerController.bShowMouseCursor` true (`GameplayStatics.GetPlayerController` null))))

(event `Update player tags when in stealth`
  ;[1 1 1] Sets the players relevant tags when they are in stealth
  (bind _asplayer_character_bp (cast `/Game/blueprints/PlayerCharacter_BP` (`GameplayStatics.GetPlayerCharacter` null)))
  (if (`self.IsInStealth`)
    (set `Actor.Tags` (`self.NotStealthTags`) _asplayer_character_bp)
    (else
      (set `Actor.Tags` (`self.StealthTags`) _asplayer_character_bp))))

(event `self.ReceiveTick`
  (params (DeltaSeconds :type "Float (single-precision)"))
  ;[1 1 1] Update the health and invisiblilty widgets on Tick
  (`self.Update player tags when in stealth`)
  (if (`self.IsDissolving`)
    (set `self.DissolveValue` (- (`self.DissolveValue`) 0.02))
    (`KismetMaterialLibrary.SetScalarParameterValue` null "/Game/Materials/DissoveCollection.DissoveCollection" "Dissolve" (`self.DissolveValue`))
    (else
      (set `self.DissolveValue` 1.0))))

(event `self.ReceiveBeginPlay`
  ;[1 1 1] Init health widget
  (`parent.ReceiveBeginPlay`)
  (bind _returnvalue (`|CreateWidget` "/Game/UI/WBP_PlayerHUD.WBP_PlayerHUD_C"))
  (`UserWidget.AddToViewport` _returnvalue 0))

(event `Key|LeftMouseButton`
  (:`Pressed`
    (bind _returnvalue (`|SpawnActorFromClass` "/Game/blueprints/TeleportGadget_BP.TeleportGadget_BP_C" (`KismetMathLibrary.MakeTransform` (`SceneComponent.K2_GetComponentLocation` (`self.Gadget`)) (`self.K2_GetActorRotation`)) true self))
    (set `self.IsDissolving` true)
    (`PrimitiveComponent.SetMaterial` (`self.Mesh`) 0 "/Game/Materials/m_Dissolve.m_Dissolve")
    (`KismetSystemLibrary.Delay` null 0.5)
    (`GameplayStatics.SpawnEmitterAtLocation` "/Game/Particles/P_Steam_Lit.P_Steam_Lit" (`self.K2_GetActorLocation`))
    (bind _returnvalue_2 (`self.K2_GetActorLocation` _returnvalue))
    (bind _returnvalue_3 (`GameplayStatics.SpawnEmitterAtLocation` null "/Game/Particles/P_Steam_Lit.P_Steam_Lit" _returnvalue_2))
    (`self.K2_DestroyActor` _returnvalue)
    (`self.K2_TeleportTo` _returnvalue_2)
    (`KismetSystemLibrary.Delay` null 0.5)
    (`ActorComponent.Deactivate` _returnvalue_3)
    (set `self.IsDissolving` false)
    (`PrimitiveComponent.SetMaterial` (`self.Mesh`) 0 "/Game/ProtoCharacters/Materials/MI_PrototypeMale.MI_PrototypeMale")))

(fn `UserConstructionScript`)