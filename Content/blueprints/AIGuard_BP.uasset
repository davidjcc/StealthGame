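; AI guard character Blueprint that follows patrol waypoints and changes pace when it has seen an enemy.
; BeginPlay and SetNextWaypoint write GuardTarget to the blackboard, with the latter also flagging it as a waypoint.
; Tick feeds Health to a widget, yaws Scene1 toward the player, and picks run or walk speed from HasSeenEnemy.
; As written, damage subtracts zero and the destroy-at-zero-health check is unconnected.
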(event `self.ReceiveBeginPlay`
  ;[1 1 1] Sets the blackboard 'GuardTarget' to the target in the world
  (`parent.ReceiveBeginPlay`)
  (`BlackboardComponent.SetValueAsObject` (`AIBlueprintHelperLibrary.GetBlackboard` self) "GuardTarget" (`self.GuardTarget`)))

(event `self.ReceiveAnyDamage`
  (params (Damage :type "Float (single-precision)") (DamageType :type "DamageType Object Reference") (InstigatedBy :type "Controller Object Reference") (DamageCauser :type "Actor Object Reference"))
  ;[1 1 1] Handles damaged taken and updated health
  (set `self.Health` (- (`self.Health`) 0.0)))

(event `self.ReceiveTick`
  (params (DeltaSeconds :type "Float (single-precision)"))
  (bind _scene1 (`self.Scene1`))
  (bind _charactermovement (`self.CharacterMovement`))
  (bind _aswbp_guard_health (cast `/Game/UI/WBP_GuardHealth` (`WidgetComponent.GetUserWidgetObject` (`self.HealthWidget`))))
  (set `/Game/UI/WBP_GuardHealth.DisplayHealth` (`self.Health`) _aswbp_guard_health)
  (`SceneComponent.K2_SetWorldRotation` _scene1 (`KismetMathLibrary.MakeRot` 0.0 (.yaw (`KismetMathLibrary.FindLookAtRotation` (`SceneComponent.K2_GetComponentLocation` _scene1) (`self.K2_GetActorLocation` (`GameplayStatics.GetPlayerCharacter` 0))))) false)
  (if (`BlackboardComponent.GetValueAsBool` (`AIBlueprintHelperLibrary.GetBlackboard` self) "HasSeenEnemy")
    (set `CharacterMovementComponent.MaxWalkSpeed` (`self.RunSpeed`) _charactermovement)
    (else
      (set `CharacterMovementComponent.MaxWalkSpeed` (`self.WalkSpeed`) _charactermovement))))

(event `self.SetNextWaypoint`
  (params (NextWaypoint :type "Actor Object Reference") (CurrentWaypoint :type "Actor Object Reference"))
  (bind _returnvalue (`AIBlueprintHelperLibrary.GetBlackboard` self))
  ;[1 1 1] Set the next waypoint in the guard patrol route
  (set `self.GuardTarget` NextWaypoint)
  (`BlackboardComponent.SetValueAsObject` _returnvalue "GuardTarget" (`self.GuardTarget`))
  (`BlackboardComponent.SetValueAsBool` _returnvalue "GuardTargetsWaypoint" true))

(fn `UserConstructionScript`)