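; Guard Blueprint for an AI that patrols a waypoint route, driven by its Blackboard.
; BeginPlay writes the initial GuardTarget to the Blackboard.
; SetNextWaypoint stores a new target, updates that key and sets the GuardTargetsWaypoint flag.
; Each tick, after the parent tick, it turns its Scene component in yaw only to face the first player's character.
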(event `self.ReceiveBeginPlay`
  ;[1 1 1] Set the first waypoint
  (`BlackboardComponent.SetValueAsObject` (`AIBlueprintHelperLibrary.GetBlackboard` self) "GuardTarget" (`self.GuardTarget`)))

(event `self.SetNextWaypoint`
  (params (NextWaypoint :type "Actor Object Reference") (CurrentWaypoint :type "Actor Object Reference"))
  (bind _returnvalue (`AIBlueprintHelperLibrary.GetBlackboard` self))
  ;[1 1 1] Set the next waypoint in the guard patrol route
  (set `self.GuardTarget` NextWaypoint)
  (`BlackboardComponent.SetValueAsObject` _returnvalue "GuardTarget" (`self.GuardTarget`))
  (`BlackboardComponent.SetValueAsBool` _returnvalue "GuardTargetsWaypoint" true))

(event `self.ReceiveTick`
  (params (DeltaSeconds :type "Float (single-precision)"))
  (bind _scene (`self.Scene`))
  (`parent.ReceiveTick` DeltaSeconds)
  (`SceneComponent.K2_SetWorldRotation` _scene (`KismetMathLibrary.MakeRot` 0.0 (.yaw (`KismetMathLibrary.FindLookAtRotation` (`SceneComponent.K2_GetComponentLocation` _scene) (`self.K2_GetActorLocation` (`GameplayStatics.GetPlayerCharacter` 0))))) false))

(fn `UserConstructionScript`)