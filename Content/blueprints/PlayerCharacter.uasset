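; Player character Blueprint that handles pause input, disguise tags, damage and HUD updates.
; Tick sets Tags from IsInDisguise, apparently inverted (disguised gets NotInDisguiseTag), and pushes health and disguise time to the HUD widget if valid.
; HUD creation is disconnected from the empty BeginPlay, so it never runs here.
; Damage forwards to PlayerTakeDamage; pause input opens WBP_PauseMenu with a cursor but calls SetGamePaused with false.
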(event `InputAction|GamePause`
  ;[1 1 1] Pause Game
  (:`Pressed`
    (`GameplayStatics.SetGamePaused` null)
    (bind _returnvalue (`|CreateWidget` "/Game/UI/WBP_PauseMenu.WBP_PauseMenu_C"))
    (`UserWidget.AddToViewport` _returnvalue)
    (set `PlayerController.bShowMouseCursor` true (`GameplayStatics.GetPlayerController` null))))

(event `Update Player Disguise Material`
  ;[1 1 1] Sets the players relevant tags when they are in digsuise
  (bind _asplayer_character (cast `/Game/blueprints/PlayerCharacter` (`GameplayStatics.GetPlayerCharacter` null)))
  (if (`self.isInDisguise`)
    (set `Actor.Tags` (`self.NotInDisguiseTag`) _asplayer_character)
    (else
      (set `Actor.Tags` (`self.DisguiseTag`) _asplayer_character))))

(event `self.ReceiveTick`
  (params (DeltaSeconds :type "Float (single-precision)"))
  (bind _playerhudwidget (`self.PlayerHudWidget`))
  ;[1 1 1] Update the health and invisiblilty widgets on Tick
  (`self.Update Player Disguise Material`)
  (`/Engine/EditorBlueprintResources/StandardMacros.IsValid` _playerhudwidget
    (:`Is Valid`
      (bind _aswbp_player_hud (cast `/Game/UI/WBP_PlayerHUD` _playerhudwidget))
      (set `/Game/UI/WBP_PlayerHUD.HealthToDisplay` (`self.PlayerHealth`) _aswbp_player_hud)
      (set `/Game/UI/WBP_PlayerHUD.DisguiseAmountToDisplay` (`self.DisguiseTime`) _aswbp_player_hud))))

(event `self.ReceiveAnyDamage`
  (params (Damage :type "Float (single-precision)") (DamageType :type "DamageType Object Reference") (InstigatedBy :type "Controller Object Reference") (DamageCauser :type "Actor Object Reference"))
  ;[1 1 1] Handle event when damage is taken
  (`self.PlayerTakeDamage` Damage))

(event `self.ReceiveBeginPlay`
  ;[1 1 1] Init health widget
)

(fn `UserConstructionScript`)